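; Player-fired projectile Blueprint that hits player characters of a different type than its own.
; SetType stores the projectile's type and recolours the Sphere with the matching Cowboy or Tennis material; construction defaults the type to NA.
; On Sphere overlap it casts to PlayerCharacterBP and, if the type is set and differs from that player's, calls IsHit with the sphere's forward vector.
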(event OnComponentBeginOverlap(Sphere)
  (params (OverlappedComponent :type Primitive%20Component%20Object%20Reference) (OtherActor :type Actor%20Object%20Reference) (OtherComp :type Primitive%20Component%20Object%20Reference) (OtherBodyIndex :type Integer) (bFromSweep :type Boolean) (SweepResult :type Hit%20Result%20Structure%20%28by%20ref%29))
  (bind _projectiletype (Variables|Default|GetProjectileType))
  (bind _asplayer_character_bp (Utilities|Casting|CastToPlayerCharacterBP OtherActor))
  (bind _playertype (Default|GetPlayerType _asplayer_character_bp))
  (if (and (Utilities|Enum|NotEqual(Enum) _projectiletype "NewEnumerator2") (!= _projectiletype _playertype))
    (Default|IsHit _asplayer_character_bp (Math|Vector|GetForwardVector (Variables|Default|GetSphere)))))

(event EventBeginPlay)

(event Collision|EventActorBeginOverlap
  (params (OtherActor :type Actor%20Object%20Reference)))

(event EventTick
  (params (DeltaSeconds :type Float%20%28single-precision%29)))

(fn ConstructionScript
  (Variables|Default|SetProjectileType "NewEnumerator2"))

(fn SetType
  (params (InType :type PlayerType%20Enum :default "NewEnumerator0"))
  (Variables|Default|SetProjectileType InType)
  (CallFunction|SetAttributes))

(fn SetAttributes
  (switch Utilities|FlowControl|Switch|SwitchonPlayerType (Variables|Default|GetProjectileType)
    (:NewEnumerator0
      (Rendering|Material|SetMaterial (Variables|Default|GetSphere) 0 "/Game/Materials/CowboyCol.CowboyCol"))
    (:NewEnumerator1
      (Rendering|Material|SetMaterial (Variables|Default|GetSphere) 0 "/Game/Materials/TennisCol.TennisCol"))))