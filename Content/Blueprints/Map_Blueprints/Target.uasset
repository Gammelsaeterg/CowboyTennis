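; Target actor that travels along a spline path and, when shot, removes a tile from the ground of the side opposing the shooter.
; On BeginPlay it picks a random mesh and speed, then each tick advances time along the spline and takes that transform.
; Overlap with a player projectile plays an explosion sound, calls DeleteTile on the Cowboy or Tennis ground opposite the projectile's type, then destroys both actors.
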(event EventBeginPlay
  (bind _possible_meshes (Variables|Default|GetPossible%20Meshes))
  (Components|StaticMesh|SetStaticMesh (Variables|Default|GetStaticMesh) (Utilities|Array|Get(acopy) _possible_meshes (Math|Random|RandomIntegerinRange 0 (- (Utilities|Array|Length _possible_meshes) 1))))
  (Variables|Default|SetSpeed (Math|Random|RandomFloatinRange 0.1 0.25)))

(event Collision|EventActorBeginOverlap
  (params (OtherActor :type Actor%20Object%20Reference))
  (bind _asplayer_projectile_bp (Utilities|Casting|CastToPlayerProjectileBP OtherActor))
  (Audio|PlaySoundatLocation "/Game/Assets/Sounds/Explosion.Explosion" (Transformation|GetActorLocation) "0, 0, 0" 1.0 1.0 0.0 0 0 0)
  (switch Utilities|FlowControl|Switch|SwitchonPlayerType (Variables|/Game/Blueprints/PlayerProjectileBP.PlayerProjectileBP_C|GetProjectileType _asplayer_projectile_bp)
    (:NewEnumerator0
      (Default|DeleteTile (Utilities|ResolveSoftReference (Variables|Default|GetTennisGround))))
    (:NewEnumerator1
      (Default|DeleteTile (Utilities|ResolveSoftReference (Variables|Default|GetCowboyGround)))))
  (Actor|DestroyActor)
  (Actor|DestroyActor _asplayer_projectile_bp))

(event EventTick
  (params (DeltaSeconds :type Float%20%28single-precision%29))
  (bind _output_get (Variables|Default|Sett (+ (Variables|Default|Gett) (* DeltaSeconds (Variables|Default|GetSpeed)))))
  (Transformation|SetActorTransform (Spline|GetTransformatTime (Variables|/Game/Blueprints/Map_Blueprints/Path.Path_C|GetSpline (Variables|Default|GetPath)) _output_get "World" false false)))

(fn ConstructionScript)