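; Path is a spline actor that repeatedly spawns Target actors for the map.
; Tick runs a random Delay between MinSpawnTime and MaxSpawnTime, then calls SpawnTarget, so the latent node paces the spawning.
; SpawnTarget places each Target at a world-space spline transform and passes itself as that Target's Path reference.
; BeginPlay also calls SetTimerByFunctionName, with no function name shown.
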(event EventBeginPlay
  (Utilities|Time|SetTimerbyFunctionName 0 "" 0.0))

(event Collision|EventActorBeginOverlap
  (params (OtherActor :type Actor%20Object%20Reference)))

(event EventTick
  (params (DeltaSeconds :type Float%20%28single-precision%29))
  (Utilities|FlowControl|Delay (Math|Random|RandomFloatinRange (Variables|Default|GetMin%20Spawn%20Time) (Variables|Default|GetMax%20Spawn%20Time)))
  (CallFunction|SpawnTarget))

(fn ConstructionScript)

(fn SpawnTarget
  (bind _returnvalue (Game|SpawnActorfromClass "/Game/Blueprints/Map_Blueprints/Target.Target_C" (Spline|GetTransformatTime (Variables|Default|GetSpline) 0.0 "World" false false) "Undefined" 0 0))
  (Variables|/Game/Blueprints/Map_Blueprints/Target.Target_C|SetPath _returnvalue self))