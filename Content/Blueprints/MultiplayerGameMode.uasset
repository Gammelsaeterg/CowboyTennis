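; Game mode that spawns and sets up local multiplayer players when play begins.
; It gathers all PlayerStarts, then for each index below MaxPlayerCount creates a local player at every start whose PlayerStartTag matches that index.
; Each spawned PlayerCharacterBP is possessed by that index's controller, given its index and one of two player types, and added to the Players list.
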(event EventBeginPlay
  (CallFunction|GetPlayerStartPoints)
  (CallFunction|SpawnPlayers))

(fn ConstructionScript)

(fn GetPlayerStartPoints
  (bind _outactors (Actor|GetAllActorsOfClass "/Script/Engine.PlayerStart"))
  (Variables|Default|SetPlayerStartArray _outactors))

(fn SpawnPlayers
  (for _index (range 0 (- (Variables|Default|GetMaxPlayerCount) 1))
    (Variables|Default|SetIndex _index)
    (for _array_element (Variables|Default|GetPlayerStartArray)
      (if (Utilities|Enum|Equal(Enum) (Utilities|String|ToString(Name) (Variables|/Script/Engine.PlayerStart|GetPlayerStartTag _array_element)) (Utilities|String|ToString(Integer) (Variables|Default|GetIndex)))
        (Class|GameplayStatics|CreatePlayer (Variables|Default|GetIndex))
        (bind _returnvalue (Game|SpawnActorfromClass "/Game/Blueprints/PlayerCharacterBP.PlayerCharacterBP_C" (Transformation|GetActorTransform _array_element) "AlwaysSpawn" 0 0))
        (Pawn|Possess (Game|GetPlayerController (Variables|Default|GetIndex)) _returnvalue)
        (Default|SetPlayerIndexandRot _returnvalue (Variables|Default|GetIndex))
        (bind _asplayer_character_bp (Utilities|Casting|CastToPlayerCharacterBP (Pawn|GetControlledPawn (Game|GetPlayerController (Variables|Default|GetIndex)))))
        (Default|SetPlayerType _asplayer_character_bp (Utilities|Select :Index (Variables|Default|GetIndex) :Option%200 "NewEnumerator0" :Option%201 "NewEnumerator1"))
        (Utilities|Array|AddUnique (Variables|Default|GetPlayers) _returnvalue)))))